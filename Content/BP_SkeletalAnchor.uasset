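; BP_SkeletalAnchor is a named anchor actor associated with a controlled skeletal mesh, with a separate display component to show it.
; Each tick it places AnchorDisplay at the AnchorMesh location, offset against the right vector of the mesh's pelvis socket.
; Control changes set the display's visibility from ControlEnabled, and refreshing scales AnchorMesh from AnchorRadius.
; BeginPlay prints the anchor name, while the attach event is empty.
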(event EventBeginPlay
  (Development|PrintString (Utilities|String|ToString(Name) (Variables|Default|GetAnchorName))))

(event Collision|EventActorBeginOverlap
  (params (OtherActor :type Actor%20Object%20Reference)))

(event EventTick
  (params (DeltaSeconds :type Float%20%28single-precision%29))
  (Transformation|SetWorldLocation (Variables|Default|GetAnchor%20Display) (- (Transformation|GetWorldLocation (Variables|Default|GetAnchorMesh)) (* (Math|Vector|GetRightVector (Transformation|GetSocketRotation (Variables|Default|GetControlledMesh) "pelvis")) 2e+01)) false false))

(event EventOnEnableControl
  (Rendering|SetVisibility (Variables|Default|GetAnchor%20Display) (Variables|Default|GetbControlEnabled) true))

(event EventOnAttachAnchor)

(event EventRefreshAnchorActor
  (Transformation|SetWorldScale3D (Variables|Default|GetAnchorMesh) (Math|Conversions|ToVector(Float) (/ (Variables|Default|GetAnchorRadius) 2e+02))))

(fn ConstructionScript)